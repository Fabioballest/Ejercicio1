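; Trigger button actor that reports whether something is overlapping it.
; Begin and end overlap set the Inttrigger flag and feed a shared branch, with no filter on the overlapping actor.
; The branch toggles the TextRender's visibility either way, then calls ButtonTrue on enter or ButtonFalse on exit, apparently event dispatchers for other Blueprints.
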(event EventBeginPlay)

(event EventTick
  (params (DeltaSeconds :type Float%20%28single-precision%29)))

(event Collision|EventActorBeginOverlap
  (params (OtherActor :type Actor%20Object%20Reference))
  (Variables|Default|Setinttrigger true)
  (if (Variables|Default|Getinttrigger)
    (Rendering|ToggleVisibility (Variables|Default|GetTextRender) false)
    (Default|CallButtonTrue)
    (else
      (Rendering|ToggleVisibility (Variables|Default|GetTextRender) false)
      (Default|CallButtonFalse))))

(event Collision|EventActorEndOverlap
  (params (OtherActor :type Actor%20Object%20Reference))
  (Variables|Default|Setinttrigger false)
  (if (Variables|Default|Getinttrigger)
    (Rendering|ToggleVisibility (Variables|Default|GetTextRender) false)
    (Default|CallButtonTrue)
    (else
      (Rendering|ToggleVisibility (Variables|Default|GetTextRender) false)
      (Default|CallButtonFalse))))

(fn ConstructionScript)