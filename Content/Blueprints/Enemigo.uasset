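; Enemy character that shoots, chases the player on sight and dies when its health runs out.
; A looping timer spawns BalaEnemigo bullets with a firing sound, whether or not the player is seen.
; Tick yaws the body and health-bar widget toward the player, updates the bar and destroys the actor at zero health.
; PawnSensing triggers AIMoveTo toward the player, and FirstPersonProjectile hits subtract health.
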(event OnSeePawn(PawnSensing)
  (params (Pawn :type Pawn%20Object%20Reference))
  ;[1 1 1] Movimiento enemigo cuando nos ve
  (bind _asfirst_person_character (Utilities|Casting|CastToFirstPersonCharacter Pawn))
  (AI|AIMoveTo self "0, 0, 0" _asfirst_person_character 1e+01 false))

(event EventTick
  (params (DeltaSeconds :type Float%20%28single-precision%29))
  ;[1 1 1] Barra estado enemigo
  (CallFunction|RotatetoCharacter)
  (if (<= (Variables|Default|GetSalud) 0.0)
    (Actor|DestroyActor)
    (else
      (bind _asbp_salud_enemigo (Utilities|Casting|CastToBP_SaludEnemigo (UserInterface|GetUserWidgetObject (Variables|Default|GetWidget))))
      (Progress|SetPercent (Variables|/Game/Blueprints/Widgets/BP_SaludEnemigo.BP_SaludEnemigo_C|GetProgressBar_222 _asbp_salud_enemigo) (/ (Variables|Default|GetSalud) 1e+02))
      (Transformation|SetWorldRotation (Variables|Default|GetWidget) (Math|Rotator|MakeRotator 0.0 0.0 (.Yaw (Math|Rotator|BreakRotator (Math|Rotator|FindLookatRotation (Transformation|GetWorldLocation (Variables|Default|GetWidget)) (Transformation|GetActorLocation (Game|GetPlayerCharacter 0)))))) false false))))

(event EventBeginPlay
  (Utilities|FlowControl|Sequence
    (:then_0
      (Transformation|AttachComponentToComponent (Variables|Default|GetGunMesh) (Variables|Character|GetMesh) "hand_rSocket" "SnapToTarget" "SnapToTarget" "SnapToTarget" true)
      (Animation|PlayAnimMontage "/Game/Models/Character/Animations/FirstPersonFire_Montage.FirstPersonFire_Montage" 1.0 "None"))
    (:then_1
      (Utilities|Time|SetTimerbyFunctionName 0 "Shoot_Main_Character" (Variables|Default|GetFire%20Time%20Interval) true))))

(event Collision|EventHit
  (params (MyComp :type Primitive%20Component%20Object%20Reference) (Other :type Actor%20Object%20Reference) (OtherComp :type Primitive%20Component%20Object%20Reference) (bSelfMoved :type Boolean) (HitLocation :type Vector :default "0, 0, 0") (HitNormal :type Vector :default "0, 0, 0") (NormalImpulse :type Vector :default "0, 0, 0") (Hit :type Hit%20Result%20Structure%20%28by%20ref%29))
  ;[1 1 1] Disminuir vida cuando es golpeado
  (Utilities|Casting|CastToFirstPersonProjectile Other)
  (bind _asenemigo (Utilities|Casting|CastToEnemigo (.HitActor (Collision|BreakHitResult Hit))))
  (Variables|Enemigo_C|SetSalud _asenemigo (- (Variables|Enemigo_C|GetSalud _asenemigo) 25.0)))

(fn ConstructionScript)

(fn ShootMainCharacter
  (bind _returnvalue (Transformation|GetActorTransform))
  (bind (_location _rotation) (Math|Transform|BreakTransform _returnvalue))
  (Game|SpawnActorfromClass "/Game/Blueprints/BalaEnemigo.BalaEnemigo_C" (Math|Transform|MakeTransform (+ _location "0.000000,0.000000,50.000000") _rotation) "AdjustIfPossibleButDontSpawnIfColliding" 0 0)
  (Audio|PlaySoundatLocation "/Game/Audio/FirstPersonTemplateWeaponFire02.FirstPersonTemplateWeaponFire02" (Transformation|GetActorLocation) "0, 0, 0" 0.5))

(fn RotatetoCharacter
  (bind _asfirst_person_character (Utilities|Casting|CastToFirstPersonCharacter (Game|GetPlayerCharacter 0)))
  (bind _return_value (CallFunction|GetLookatRotation self _asfirst_person_character))
  (Transformation|SetActorRotation _return_value))

(fn GetLookatRotation
  (params (My%20Actor :type Actor%20Object%20Reference) (Target :type Actor%20Object%20Reference))
  (return (Math|Interpolation|RInterpTo (Transformation|GetActorRotation My%20Actor) (Math|Rotator|MakeRotator 0.0 0.0 (.Yaw (Math|Rotator|BreakRotator (Math|Rotator|FindLookatRotation (Transformation|GetActorLocation My%20Actor) (Transformation|GetActorLocation Target))))) (Utilities|Time|GetWorldDeltaSeconds) 0.0)))